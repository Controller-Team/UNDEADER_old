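; Weapon system for the third-person player character, providing helpers for equipping, ammo, montages and firing feedback.
; InitWeapon stores the weapon class and type, then sets and socket-attaches the character's pistol or rifle child actor component.
; FireCheck deducts ammo when available, while Reload resets it to ClipAmmo without touching any reserve.
; Separate functions spawn sound, muzzle and impact Niagara effects, tracer actors and decals; hit detection lives elsewhere.
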(event Custom|InitWeapon
  (params (MasterWeapon :type BP%20Master%20Weapon%20Class%20Reference) (WeaponType :type Equipt_State%20Enum :default "NewEnumerator4") (bEquiptToggle :type Boolean) (AttachSocketName :type Name))
  (Variables|Default|SetMaster%20Weapon MasterWeapon)
  (Variables|Editable|SetWeaponType WeaponType)
  (if bEquiptToggle
    _
    (else
      _))
  (CallFunction|AttachWeapon AttachSocketName (Variables|Editable|GetWeaponType)))

(event EventBeginPlay
  (bind _asbp_third_person_character (Utilities|Casting|CastToBP_ThirdPersonCharacter (Game|GetPlayerCharacter 0)))
  (Variables|Default|SetCharacterRef _asbp_third_person_character))

(fn PlaySFX
  (params (Sound :type Sound%20Base%20Object%20Reference) (ConcurrencySettings :type Sound%20Concurrency%20Object%20Reference))
  (Audio|PlaySound2D Sound 1.0 1.0 0.0 ConcurrencySettings 0 false))

(fn MuzzleVFX
  (params (SystemTemplate :type Niagara%20System%20Object%20Reference) (AttachToComponent :type Scene%20Component%20Object%20Reference))
  (Niagara|SpawnSystemAttached SystemTemplate AttachToComponent "None" "0, 0, 0" "0, 0, 0" "KeepRelativeOffset" false))

(fn ImpactVFX
  (params (Impact%20Location :type Vector) (Normal :type Vector) (Physic%20Mat :type Physical%20Material%20Object%20Reference))
  (Utilities|IsValid Physic%20Mat
    (:Is%20Valid
      (Niagara|SpawnSystematLocation (Utilities|Select :Index (Variables|/Script/PhysicsCore.PhysicalMaterial|GetSurfaceType Physic%20Mat) :SurfaceType_Default "/Game/Weapons/Effects/Particles/Impacts/NS_Imacts.NS_Imacts" :SurfaceType1 "/Game/Weapons/Effects/Particles/Impacts/NS_Imacts.NS_Imacts") Impact%20Location (Math|Conversions|RotationFromXVector Normal)))))

(fn BulletTrace
  (params (Socket%20Location :type Vector) (Location :type Vector) (End :type Vector))
  (Game|SpawnActorfromClass "/Game/Weapons/BulletTrace/Bullet_Trace.Bullet_Trace_C" (Math|Transform|MakeTransform Socket%20Location (Math|Rotator|FindLookatRotation Location End)) "Undefined" "OverrideRootScale" 0 0))

(fn ImpactDecal
  (params (Class :type Actor%20Class%20Reference) (Location :type Vector) (Normal :type Vector) (Scale :type Vector))
  (Game|SpawnActorfromClass Class (Math|Transform|MakeTransform Location (Math|Conversions|RotationFromXVector Normal) Scale) "Undefined" "SelectDefaultAtRuntime" 0 0))

(fn FireCheck
  (bind _weapon_details (Variables|Editable|GetWeapon_Details))
  (bind _weapon_data (Utilities|Struct|BreakWeapon_Details _weapon_details))
  (bind (_currentammo _maxammo _ammo_count) (Utilities|Struct|BreakWeapon_Data _weapon_data))
  (LocalVariables|SetWeaponDataRef (Utilities|Struct|BreakWeapon_Details (Variables|Editable|GetWeapon_Details)))
  (if (>= _currentammo 1) ; 탄환이 한발이라도 있다면
    (Utilities|Struct|SetmembersinWeapon_Data (Utilities|Struct|BreakWeapon_Details (Variables|Editable|GetWeapon_Details)) (Math|Integer|Clamp(Integer) (- _currentammo _ammo_count) 0 _maxammo))
    (return true)
    (else
      (return false))))

(fn Reload
  (bind _weapon_details (Variables|Editable|GetWeapon_Details))
  (bind _weapon_data (Utilities|Struct|BreakWeapon_Details _weapon_details))
  (Utilities|Struct|SetmembersinWeapon_Data _weapon_data (.ClipAmmo (Utilities|Struct|BreakWeapon_Data _weapon_data)))
  (return))

(fn PlayMontage
  (params (MontageToPlay :type Anim%20Montage%20Object%20Reference))
  (bind _returnvalue (Animation|Montage|MontagePlay (Components|SkeletalMesh|GetAnimInstance (Variables|/Script/Engine.Character|GetMesh (Variables|Default|GetCharacterRef))) MontageToPlay 1.0 "Duration" 0.0 true))
  (Development|PrintString (Utilities|GetDisplayName MontageToPlay))
  (return _returnvalue))

(fn AttachWeapon
  (params (SocketName :type Name) (weaponType :type Equipt_State%20Enum :default "NewEnumerator4"))
  (bind _characterref (Variables|Default|GetCharacterRef))
  (LocalVariables|Set_SocketName SocketName)
  (switch Utilities|FlowControl|Switch|SwitchonEquipt_State weaponType
    (:NewEnumerator4
      (Development|PrintString "attach weapon : unarmed!"))
    (:NewEnumerator5
      (LocalVariables|SetTargetChildActor (Variables|/Game/Blueprints/PlayerCharacter/BP_ThirdPersonCharacter.BP_ThirdPersonCharacter_C|GetPistolChild _characterref))
      (ChildActorComponent|SetChildActorClass (LocalVariables|GetTargetChildActor) (Variables|Default|GetMaster%20Weapon) :!label _label)
      (Transformation|AttachComponentToComponent (LocalVariables|GetTargetChildActor) (Variables|/Script/Engine.Character|GetMesh (Variables|Default|GetCharacterRef)) (LocalVariables|Get_SocketName) "SnapToTarget" "SnapToTarget" "SnapToTarget" true))
    (:NewEnumerator6
      (LocalVariables|SetTargetChildActor (Variables|/Game/Blueprints/PlayerCharacter/BP_ThirdPersonCharacter.BP_ThirdPersonCharacter_C|GetRifleChild _characterref))
      (goto _label))))