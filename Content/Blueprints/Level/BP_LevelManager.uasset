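; Level manager that runs the escape countdown and handles level transitions.
; On BeginPlay it caches HUD and fade widgets from the game mode, disables all escape areas, fades in, and zeroes the timer on the start level.
; Tick updates the HUD countdown and re-enables every BP_EscapeArea each frame once the whole-second value reaches zero.
; ToNextLevel fades out, increments the GameInstance level counter and opens the matching level.
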(event Custom|ToNextLevel
  (bind _duration (Default|DoFade (Variables|Default|GetWBP%20Fade) "Reverse"))
  (Utilities|FlowControl|Delay _duration)
  (bind _currlevel (Default|LevelCountUp (Variables|Default|GetAs%20GI%20Undeader)))
  (Development|PrintString (Utilities|String|Append "lvl: " (Utilities|String|ToString(Integer) _currlevel)) true true "(R=1.000000,G=0.084749,B=0.000000,A=1.000000)" 99.0)
  (switch int (Default|GetCurrLevel (Variables|Default|GetAs%20GI%20Undeader))
    (:1
      (Game|OpenLevel(byObjectReference) (Variables|Editable|GetLevel1)))
    (:2
      (Game|OpenLevel(byObjectReference) (Variables|Editable|GetLevel2)))
    (:3
      (Game|OpenLevel(byObjectReference) (Variables|Editable|GetLevel3)))))

(event Custom|ToggleAllEscapeArea
  (params (toggle :type Boolean))
  (bind _outactors (Actor|GetAllActorsOfClass "/Game/Blueprints/Level/BP_EscapeArea.BP_EscapeArea_C"))
  (for _array_element _outactors
    (Default|ToggleAllEscapeArea _array_element toggle)))

(event EventBeginPlay
  (Utilities|FlowControl|Sequence
    (:then_0
      (bind _asbp_third_person_game_mode (Utilities|Casting|CastToBP_ThirdPersonGameMode (Game|GetGameMode)))
      (Variables|Default|SetWBP%20HUD (Variables|/Game/Blueprints/BP_ThirdPersonGameMode.BP_ThirdPersonGameMode_C|GetWBP%20HUD _asbp_third_person_game_mode))
      (Variables|Default|SetWBP%20Fade (Variables|/Game/Blueprints/BP_ThirdPersonGameMode.BP_ThirdPersonGameMode_C|GetWBP%20Fade _asbp_third_person_game_mode))
      (bind _asgi_undeader (Utilities|Casting|CastToGI_Undeader (Game|GetGameInstance))
        (:then
          (Variables|Default|SetAs%20GI%20Undeader _asgi_undeader))
        (:CastFailed
          (Development|PrintString "Hello???"))))
    (:then_1
      (CallFunction|ToggleAllEscapeArea false)
      (Default|DoFade (Variables|Default|GetWBP%20Fade) "Forward"))
    (:then_2
      (if (CallFunction|IsStartLevel)
        (Variables|Editable|SetLeftEscapeTime 0.0)))))

(event EventTick
  (params (DeltaSeconds :type Float%20%28single-precision%29))
  (bind _output_get (Variables|Editable|SetLeftEscapeTime (Math|Float|Clamp(Float) (- (Variables|Editable|GetLeftEscapeTime) DeltaSeconds) 0.0 99.0)))
  (Default|SetRemainTime (Variables|Default|GetWBP%20HUD) (Math|Float|Truncate _output_get))
  (if (== (Math|Float|Truncate _output_get) 0)
    (CallFunction|ToggleAllEscapeArea true)))

(fn ConstructionScript)

(fn IsStartLevel
  (return (== (Default|GetCurrLevel (Variables|Default|GetAs%20GI%20Undeader)) 0)))