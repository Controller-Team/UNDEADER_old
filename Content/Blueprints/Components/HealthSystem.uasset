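; Health component that tracks an owner's current and maximum health and its death state.
; InitHealthSystem sets the maximum, fills current health to it and broadcasts an init dispatcher.
; AdjustHealth applies a signed change clamped between zero and maximum, broadcasts it, then runs DeadCheck, which sets Dead and fires the death dispatcher at zero health.
; GetPercent returns current health divided by maximum.
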(event Custom|AdjustHealth
  (params (adjust :type Integer))
  (Variables|Default|SetCurrHealth (Math|Integer|Clamp(Integer) (+ (Variables|Default|GetCurrHealth) adjust) 0 (Variables|Default|GetMaxHealth)))
  (Default|CallOnAdjustHealthEventDispatcher)
  (CallFunction|DeadCheck))

(event Custom|InitHealthSystem
  (params (MaxHealth :type Integer))
  (bind _output_get (Variables|Default|SetMaxHealth MaxHealth))
  (Variables|Default|SetCurrHealth _output_get)
  (Default|CallOnInitEventDispatcher))

(fn GetPercent
  (return (/ (Variables|Default|GetCurrHealth) (Variables|Default|GetMaxHealth))))

(fn DeadCheck
  (bind _output_get (Variables|Default|SetbDead? (<= (Variables|Default|GetCurrHealth) 0)))
  (if _output_get
    (Default|CallOnDeadEventDispatcher)))