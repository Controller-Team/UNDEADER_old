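; StaminaSystem is a component Blueprint that tracks an integer stamina pool, set to full when InitStamina supplies the maximum.
; UseStamina deducts a cost through AdujstStamina when enough remains, returning false on success and true when stamina is insufficient.
; AdujstStamina clamps the value between zero and the maximum, then fires the AdjustStaminaED dispatcher, while initialization does not broadcast.
; A getter exposes the current value.
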(event Custom|InitStamina
  (params (MaxStamina :type Integer))
  (bind _output_get (Variables|Default|SetMaxStamina MaxStamina))
  (Variables|Default|SetCurrStamin _output_get))

(fn UseStamina
  (params (Usage :type Integer))
  (if (>= (Variables|Default|GetCurrStamin) Usage)
    (CallFunction|AdujstStamina (* Usage -1))
    (return false)
    (else
      (return true))))

(fn AdujstStamina
  (params (adjust :type Integer))
  (Variables|Default|SetCurrStamin (Math|Integer|Clamp(Integer) (+ adjust (Variables|Default|GetCurrStamin)) 0 (Variables|Default|GetMaxStamina)))
  (Default|CallAdjustStaminaED))

(fn GetCurrStamina
  (return (Variables|Default|GetCurrStamin)))