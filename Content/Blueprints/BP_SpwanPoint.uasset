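; Spawn point actor that tests whether its bounding box is on screen for the first player, currently as a debug readout.
; BeginPlay caches the box corners from the actor's bounds via GetCorners.
; Each Tick, CheckVisible projects them to widget coordinates, passing if any lands within twice the viewport size, with no occlusion test.
; Tick prints the result and draws debug spheres at the corners; no spawning logic exists here.
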(event Custom|InitBound
  (params (ActorToCheckBounds :type Actor%20Object%20Reference))
  (bind (_origin _boxextent) (Collision|GetActorBounds ActorToCheckBounds false false))
  (Variables|Default|SetCorners (CallFunction|GetCorners _origin _boxextent)))

(event EventBeginPlay
  (CallFunction|InitBound self))

(event EventTick
  (params (DeltaSeconds :type Float%20%28single-precision%29))
  (bind _visible (CallFunction|CheckVisible (Variables|Default|GetCorners)))
  (Development|PrintString (Utilities|String|ToString(Boolean) _visible))
  (for _array_element (Variables|Default|GetCorners)
    (Rendering|Debug|DrawDebugSphere _array_element 1e+01 6 "(R=1.000000,G=1.000000,B=1.000000,A=1.000000)" 0.0)))

(fn ConstructionScript)

(fn GetCorners
  (params (Origin :type Vector) (BoxExtent :type Vector))
  (LocalVariables|Setm_Origin Origin)
  (LocalVariables|Setm_BoxExtent BoxExtent)
  (Utilities|FlowControl|Sequence
    (:then_0
      (LocalVariables|Setmin (- (LocalVariables|Getm_Origin) (LocalVariables|Getm_BoxExtent)))
      (LocalVariables|Setmax (+ (LocalVariables|Getm_Origin) (LocalVariables|Getm_BoxExtent))))
    (:then_1
      (LocalVariables|SetVecs (Utilities|Array|MakeArray (LocalVariables|Getmin) (LocalVariables|Getmax))))
    (:then_2
      (Utilities|Array|Add (LocalVariables|GetVecs) (Math|Vector|MakeVector (.x (LocalVariables|Getmin)) (.y (LocalVariables|Getmin)) (.z (LocalVariables|Getmax))))
      (Utilities|Array|Add (LocalVariables|GetVecs) (Math|Vector|MakeVector (.x (LocalVariables|Getmin)) (.y (LocalVariables|Getmax)) (.z (LocalVariables|Getmax))))
      (Utilities|Array|Add (LocalVariables|GetVecs) (Math|Vector|MakeVector (.x (LocalVariables|Getmax)) (.y (LocalVariables|Getmin)) (.z (LocalVariables|Getmax))))
      (Utilities|Array|Add (LocalVariables|GetVecs) (Math|Vector|MakeVector (.x (LocalVariables|Getmax)) (.y (LocalVariables|Getmax)) (.z (LocalVariables|Getmax)))))
    (:then_3
      (Utilities|Array|Add (LocalVariables|GetVecs) (Math|Vector|MakeVector (.x (LocalVariables|Getmin)) (.y (LocalVariables|Getmin)) (.z (LocalVariables|Getmin))))
      (Utilities|Array|Add (LocalVariables|GetVecs) (Math|Vector|MakeVector (.x (LocalVariables|Getmin)) (.y (LocalVariables|Getmax)) (.z (LocalVariables|Getmin))))
      (Utilities|Array|Add (LocalVariables|GetVecs) (Math|Vector|MakeVector (.x (LocalVariables|Getmax)) (.y (LocalVariables|Getmin)) (.z (LocalVariables|Getmin))))
      (Utilities|Array|Add (LocalVariables|GetVecs) (Math|Vector|MakeVector (.x (LocalVariables|Getmax)) (.y (LocalVariables|Getmax)) (.z (LocalVariables|Getmin)))))
    (:then_4
      (return (LocalVariables|GetVecs)))))

(fn CheckVisible
  (params (Bound%20Corners :type Array%20of%20Vectors))
  (bind _returnvalue (Viewport|GetViewportSize))
  (bind _returnvalue_2 (* _returnvalue 2.0))
  (bind _array_element (Utilities|Array|ForEachLoopwithBreak Bound%20Corners)
    (:LoopBody
      (if (and (Math|Float|InRange(Float) (.X (Math|Vector2D|BreakVector2D (.ScreenPosition (Class|WidgetLayoutLibrary|ProjectWorldLocationtoWidgetPosition (Game|GetPlayerController 0) _array_element true)))) 0.0 (.x _returnvalue_2)) (Math|Float|InRange(Float) (.Y (Math|Vector2D|BreakVector2D (.ScreenPosition (Class|WidgetLayoutLibrary|ProjectWorldLocationtoWidgetPosition (Game|GetPlayerController 0) _array_element true)))) 0.0 (.y _returnvalue_2)))
        (return true)))
    (:Completed
      (return false))))