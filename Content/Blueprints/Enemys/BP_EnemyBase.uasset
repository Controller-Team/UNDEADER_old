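; Base enemy character that chases the player, plays a zombie attack montage in range and ragdolls on death.
; Tick reissues AIMoveTo toward the player while alive, or to its own location while attacking.
; A box overlap on the player triggers attacks, with an Attacking flag mirrored to ABP_Enemy until the montage delay ends.
; A HealthSystem component drives the health gauge widget and dispatches death.
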(event Custom|FollowPlayer
  (AI|AIMoveTo self (Transformation|GetActorLocation (Game|GetPlayerCharacter 0)) 0 5.0 false))

(event Custom|AttackCheck
  (bind _in_play_rate (Variables|Default|GetIn%20Play%20Rate))
  (if (not (Variables|Default|GetbAttacking?))
    (Development|PrintString "attack")
    (CallFunction|SetAttacking true)
    (bind _returnvalue (Animation|PlayAnimMontage "/Game/BSP_ZombieAnims/Animations/Standing/Attack/AM_zombieAttack.AM_zombieAttack" _in_play_rate "None"))
    (Utilities|FlowControl|Delay (/ _returnvalue _in_play_rate))
    (CallFunction|SetAttacking false)))

(event Custom|OnDead
  (bind _mesh (Variables|Character|GetMesh))
  (Collision|SetCollisionEnabled _mesh "PhysicsOnly")
  (Physics|SetSimulatePhysics _mesh true)
  (Default|ToggleHealthUI (Variables|Default|GetHealthSystem) false)
  (Collision|SetCollisionEnabled (Variables|Collision|GetCapsuleComponent) "NoCollision"))

(event Custom|SetAttacking
  (params (ShouldAttack :type Boolean))
  (bind _output_get (Variables|Default|SetbAttacking? ShouldAttack))
  (bind _asabp_enemy (Utilities|Casting|CastToABP_Enemy (Components|SkeletalMesh|GetAnimInstance (Variables|Character|GetMesh))))
  (Variables|/Game/Blueprints/Enemys/ABP_Enemy.ABP_Enemy_C|SetShouldAttack _asabp_enemy _output_get))

(event Custom|InitHealthSystem
  (Utilities|FlowControl|Sequence
    (:then_0
      (bind _aswbp_health_gage (Utilities|Casting|CastToWBP_HealthGage (UserInterface|GetWidget (Variables|Default|GetHealthGage))))
      (Default|InitHealthSystem (Variables|Default|GetHealthSystem) 0 _aswbp_health_gage))
    (:then_1
      (EventDispatchers|BindEventtoOnDeadEventDispatcher (Variables|Default|GetHealthSystem) (delegate Custom|OnDead)))))

(event EventBeginPlay
  (CallFunction|InitHealthSystem)
  (Variables|/Script/Engine.CharacterMovementComponent|SetMaxWalkSpeed (Variables|Character|GetCharacterMovement) (Variables|Default|GetMoveSpeedMax)))

(event EventTick
  (params (DeltaSeconds :type Float%20%28single-precision%29))
  (Utilities|FlowControl|Sequence
    (:then_0
      (Utilities|TargetinRange "/Game/Blueprints/PlayerCharacter/BP_PlayerCharacter.BP_PlayerCharacter_C"
        (:true
          (CallFunction|AttackCheck))))
    (:then_1
      (if (not (Variables|/Game/ThirdPerson/UI/HealthSystem.HealthSystem_C|GetbDead? (Variables|Default|GetHealthSystem)))
        (if (not (Variables|Default|GetbAttacking?))
          (CallFunction|FollowPlayer)
          (else
            (AI|AIMoveTo self (Transformation|GetActorLocation) 0 5.0 false)))))))

(fn ConstructionScript)

(fn GetBounds
  (bind (_origin _boxextent) (Collision|GetActorBounds false false))
  (return _origin _boxextent))