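; EnemyBase is a base enemy Blueprint that provides health setup and ragdoll death.
; On BeginPlay it passes the HealthGage component's WBP_HealthGage widget to its HealthSystem component and binds OnDead to that component's death dispatcher.
; OnDead switches the mesh to physics-only collision with simulated physics and hides the health UI.
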(event Custom|OnDead
  (bind _mesh (Variables|Character|GetMesh))
  (Collision|SetCollisionEnabled _mesh "PhysicsOnly")
  (Physics|SetSimulatePhysics _mesh true)
  (Default|ToggleHealthUI (Variables|Default|GetHealthSystem) false))

(event Custom|InitHealthSystem
  (Utilities|FlowControl|Sequence
    (:then_0
      (bind _aswbp_health_gage (Utilities|Casting|CastToWBP_HealthGage (UserInterface|GetWidget (Variables|Default|GetHealthGage))))
      (Default|InitHealthSystem (Variables|Default|GetHealthSystem) 0 _aswbp_health_gage))
    (:then_1
      (EventDispatchers|BindEventtoOnDeadEventDispatcher (Variables|Default|GetHealthSystem) (delegate Custom|OnDead)))))

(event EventBeginPlay
  (CallFunction|InitHealthSystem))

(event Collision|EventActorBeginOverlap
  (params (OtherActor :type Actor%20Object%20Reference)))

(event EventTick
  (params (DeltaSeconds :type Float%20%28single-precision%29)))

(fn ConstructionScript)